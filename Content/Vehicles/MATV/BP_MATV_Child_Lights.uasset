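; MATV vehicle child Blueprint that adds a toggle for its spotlight.
; The ToggleLights event calls an implementation that checks SpotLight1's current intensity with a float tolerance and switches it between off and full brightness, using intensity as the on/off state.
; Both SetIntensity targets in each branch are SpotLight1, so no other light is changed.
; BeginPlay is disabled, Tick and overlap are empty, and construction only calls the parent.
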(event Custom|ToggleLights_Implementation
  (bind _spotlight1 (Variables|Default|GetSpotLight1))
  (if (Math|Float|NearlyEqual(Float) (Variables|/Script/Engine.LightComponentBase|GetIntensity _spotlight1) 1e+04 1.0)
    (Rendering|Components|Light|SetIntensity _spotlight1 0.0)
    (else
      (Rendering|Components|Light|SetIntensity _spotlight1 1e+04))))

(event Custom|ToggleLights
  (CallFunction|ToggleLightsImplementation))

(event EventBeginPlay
  (|CallParentFunction))

(event Collision|EventActorBeginOverlap
  (params (OtherActor :type Actor%20Object%20Reference)))

(event EventTick
  (params (DeltaSeconds :type Float%20%28single-precision%29)))

(fn ConstructionScript
  (|CallParentFunction))