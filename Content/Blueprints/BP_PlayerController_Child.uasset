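; Player controller that gives a mod user-rebindable keys, driving actions such as toggling vehicle lights and showing the keybind menu.
; AnyKey events compare the pressed key against the CustomKeybinds array, through compare macros or stacked checks that ignore input during rebinding.
; While a rebind is pending and the menu is visible, the next key replaces the chosen entry and is saved.
; BeginPlay loads saved binds, or writes defaults when none exist or the version flag differs.
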(event EventBeginPlay
  (bind _custommodtitle (Variables|Default|GetCustomModTitle))
  (bind _returnvalue (Utilities|String|Append _custommodtitle "_CustomKeybinds"))
  (bind _returnvalue_2 (SaveGame|DoesSaveGameExist _returnvalue))
  (if _returnvalue_2
    ;[1 1 1] A previous save exists, load it and set it's contents to our CustomKeybinds array.
    (bind _returnvalue_3 (SaveGame|LoadGamefromSlot _returnvalue))
    (bind _assgo_custom_mod_keybinds (Utilities|Casting|CastToSGO_CustomModKeybinds _returnvalue_3))
    (if (Math|Boolean|Equal(Boolean) (Variables|Default|GetIsVersionChange) (Variables|/CustomModKeybinds/Blueprints/SGO_CustomModKeybinds.SGO_CustomModKeybinds_C|GetIsVersionChangeValue _assgo_custom_mod_keybinds))
      (Variables|Default|SetCustomKeybinds (Variables|/CustomModKeybinds/Blueprints/SGO_CustomModKeybinds.SGO_CustomModKeybinds_C|GetCustomKeybinds _assgo_custom_mod_keybinds))
      (else
        (Development|PrintString "A Version Change Was Detected. Resetting Custom Keybinds to Default.")
        ;[1 1 1] A save does not exist; create one, set the defaults from our playercontroller array, and save it so it can be loaded next time
        (bind _returnvalue_4 (SaveGame|CreateSaveGameObject "/CustomModKeybinds/Blueprints/SGO_CustomModKeybinds.SGO_CustomModKeybinds_C" :!label _label))
        (Variables|/CustomModKeybinds/Blueprints/SGO_CustomModKeybinds.SGO_CustomModKeybinds_C|SetCustomKeybinds _returnvalue_4 (Variables|Default|GetCustomKeybinds))
        (Variables|/CustomModKeybinds/Blueprints/SGO_CustomModKeybinds.SGO_CustomModKeybinds_C|SetIsVersionChangeValue _returnvalue_4 (Variables|Default|GetIsVersionChange))
        (SaveGame|SaveGametoSlot _returnvalue_4 _returnvalue)))
    (else
      (goto _label))))

(event Input|KeyboardEvents|AnyKey
  (params (Key :type Key%20Structure :default "AnyKey"))
  (bind _self self)
  ;[1 1 1] Show and Hide Our Widget that allows users to change these keybinds
  (:Pressed
    (Utilities|AnyKeyPressedReleasedComparebyIndex Key 0 :!label _label
      (:Pressed_Output
        (Utilities|IsValid (Variables|Default|GetKeybindsWidget_Reference)
          (:Is%20Valid
            (switch Utilities|FlowControl|Switch|SwitchonESlateVisibility (Widget|GetVisibility (Variables|Default|GetKeybindsWidget_Reference))
              (:Visible
                (Widget|SetVisibility (Variables|Default|GetKeybindsWidget_Reference) "Hidden")
                (Input|SetInputModeGameOnly _self)
                (Variables|Default|SetbShowMouseCursor false))
              (:Collapsed
                (Widget|SetVisibility (Variables|Default|GetKeybindsWidget_Reference) "Visible" :!label _label_2)
                (Input|SetInputModeGameandUI _self (Variables|Default|GetKeybindsWidget_Reference) "DoNotLock" false)
                (Variables|Default|SetbShowMouseCursor true))
              (:Hidden
                (goto _label_2))))
          (:Is%20Not%20Valid
            (bind _returnvalue (UserInterface|CreateWidget "/CustomModKeybinds/UI/Widgets/CustomModKeybindsMenu/W_CustomModKeybindsMenu_Container.W_CustomModKeybindsMenu_Container_C"))
            (Variables|Default|SetKeybindsWidget_Reference _returnvalue)
            (UserInterface|Viewport|AddtoViewport _returnvalue 99)
            (Input|SetInputModeGameandUI _self _returnvalue "DoNotLock" false)
            (Variables|Default|SetbShowMouseCursor true))))))
  (:Released
    (goto _label Released_Input)))

(event Input|KeyboardEvents|AnyKey
  (params (Key :type Key%20Structure :default "AnyKey"))
  (bind _custommodtitle (Variables|Default|GetCustomModTitle))
  (bind _returnvalue (Utilities|String|Append _custommodtitle "_CustomKeybinds"))
  ;[1 1 1] If we would like to rebind a key, accept new key, set it to our array, save it to the save file, then "consume the input" by setting isAwaitingNewKeybind to false.
  (:Pressed
    (if (Variables|Default|GetisAwaitingNewKeybind)
      (if (Widget|IsVisible (Variables|Default|GetKeybindsWidget_Reference))
        (Utilities|Array|SetArrayElem (Variables|Default|GetCustomKeybinds) (Variables|Default|GetIndexOfKeyToBeRebound) Key)
        (bind _returnvalue_2 (SaveGame|LoadGamefromSlot _returnvalue))
        (bind _assgo_custom_mod_keybinds (Utilities|Casting|CastToSGO_CustomModKeybinds _returnvalue_2))
        (Variables|/CustomModKeybinds/Blueprints/SGO_CustomModKeybinds.SGO_CustomModKeybinds_C|SetCustomKeybinds _assgo_custom_mod_keybinds (Variables|Default|GetCustomKeybinds))
        (SaveGame|SaveGametoSlot _assgo_custom_mod_keybinds _returnvalue)
        (Variables|Default|SetisAwaitingNewKeybind false)
        (else
          (Variables|Default|SetisAwaitingNewKeybind false))))))

(event Input|KeyboardEvents|AnyKey
  (params (Key :type Key%20Structure :default "AnyKey"))
  ;[1 1 1] Make sure in the deatails pane for any anykey event, uncheck "Consume Input" and "Override Parent Binding"
  (:Pressed
    (Utilities|AnyKeyPressedReleasedComparebyIndex Key 1 :!label _label))
  (:Released
    (goto _label Released_Input)))

(event Input|KeyboardEvents|AnyKey
  (params (Key :type Key%20Structure :default "AnyKey"))
  (bind _customkeybinds (Variables|Default|GetCustomKeybinds))
  ;[1 1 1] We can stack our input like this for low priority things that are fire and forget events
  (:Pressed
    (if (not (Variables|Default|GetisAwaitingNewKeybind))
      (if (== Key (Utilities|Array|Get(acopy) _customkeybinds 1))
        (Development|PrintString "Custom Action 1 Called")
        (elif (== Key (Utilities|Array|Get(acopy) _customkeybinds 2))
          (Development|PrintString "Custom Action 2 Called")
          (elif (== Key (Utilities|Array|Get(acopy) _customkeybinds 3))
            (Development|PrintString "You Boiled Your Head")))))))

(event Input|KeyboardEvents|AnyKey
  (params (Key :type Key%20Structure :default "AnyKey"))
  ;[1 1 1] Make sure in the deatails pane for any anykey event, uncheck "Consume Input" and "Override Parent Binding"
  (:Pressed
    (Utilities|AnyKeyPressedReleasedCompare Key (Utilities|Array|Get(acopy) (Variables|Default|GetCustomKeybinds) 1) :!label _label
      (:Pressed_Output
        (bind _asbp_matv_child_lights (Utilities|Casting|CastToBP_MATV_Child_Lights (Pawn|GetControlledPawn)))
        (Default|ToggleLights _asbp_matv_child_lights))))
  (:Released
    (goto _label Released_Input)))

(fn ConstructionScript
  (|CallParentFunction))